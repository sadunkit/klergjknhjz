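; Camera actor for Pokémon encounters that follows the player character and glides to a framing of the encounter.
; On BeginPlay it snaps and attaches to player 0's character; separate functions re-attach or detach it.
; BeginTransition plays a Duration-scaled timeline, lerping from the current transform toward the target location and a look-at rotation on the encounter center.
; It flags IsTransitioning but neither clears it nor detaches first.
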(event `self.ReceiveBeginPlay`
  (`self.K2_AttachToActor` (`GameplayStatics.GetPlayerCharacter` 0) "None" "SnapToTarget" "SnapToTarget" "KeepRelative")
  (`KismetSystemLibrary.PrintString` "Encounter Camera Helllooo!!!"))

(event `BeginTransition`
  (params (TargetLocation :type "Vector Structure") (EncounterCenter :type "Vector Structure"))
  (set `self.IsTransitioning` true)
  (`TimelineComponent.SetPlayRate` (`self.TransitionToEncounter`) (/ 1.0 (`self.Duration`)))
  (bind (_direction _alpha) (`Timeline|TransitionToEncounter` :!via `PlayFromStart`)
    (:`Update`
      (`self.K2_SetActorLocation` (`KismetMathLibrary.VLerp` (`self.K2_GetActorLocation`) TargetLocation _alpha))
      (`self.K2_SetActorRotation` (`KismetMathLibrary.RLerp` (`self.K2_GetActorRotation`) (`KismetMathLibrary.FindLookAtRotation` (`self.K2_GetActorLocation`) EncounterCenter) _alpha)))))

(fn `AttachToCharacter`
  (`self.K2_AttachToActor` (`GameplayStatics.GetPlayerCharacter` 0) "None" "SnapToTarget" "SnapToTarget" "KeepRelative"))

(fn `DetachFromCharacter`
  (`self.K2_DetachFromActor` "KeepWorld" "KeepWorld" "KeepWorld"))

(fn `UserConstructionScript`)