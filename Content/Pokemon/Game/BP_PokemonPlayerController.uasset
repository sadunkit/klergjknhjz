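; Player controller for the Pokeball character that switches the view between the pawn and an encounter camera.
; On BeginPlay it caches the character and its follow camera, spawns a BP_EncounterCamera and views the pawn.
; BeginEncounter starts that camera's transition using the static encounter's location and camera offset, then blends the view to it.
; Releasing key 1 returns the view to the pawn, and possession prints a debug string.
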(event `self.ReceiveBeginPlay`
  (bind _asbp_pokeball_third_person_character (cast `/Game/Pokemon/Characters/BP_Pokeball_ThirdPersonCharacter` (`self.K2_GetPawn`)))
  (bind _output_get (set `self.PokeballCharacter` _asbp_pokeball_third_person_character))
  (set `self.Follow Camera` (`PoketheballCharacter.FollowCamera` _output_get))
  (bind _returnvalue (`|SpawnActorFromClass` "/Game/Pokemon/Encounter/BP_EncounterCamera.BP_EncounterCamera_C" (`KismetMathLibrary.MakeTransform` (0.0 0.0 0.0)) "Undefined" "OverrideRootScale" null null))
  (set `self.EncounterCamera` _returnvalue)
  (`self.SetViewToPawn` 0.0))

(event `/Game/Pokemon/Game/BPI_Encounter.BeginEncounter`
  (params (TargetActor :type "/Game/Pokemon/Characters/BP_Pokeball_ThirdPersonCharacter Object Reference (by ref)") (EncounterActor :type "EncounterBase Object Reference (by ref)"))
  (bind _returnvalue (`self.K2_GetActorLocation` EncounterActor))
  (bind _asbp_encounter_static (cast `/Game/Pokemon/Encounter/BP_Encounter_Static` EncounterActor))
  (`/Game/Pokemon/Encounter/BP_EncounterCamera.BeginTransition` (`self.EncounterCamera`) (+ (`/Game/Pokemon/Encounter/BP_Encounter_Static.CameraLocation` _asbp_encounter_static) _returnvalue) _returnvalue)
  (`self.SetViewToEncounterCamera`))

(event `SetViewToPawn`
  (params (BlendTime :type "Float (double-precision)"))
  (`self.SetViewTargetWithBlend` self (`self.PokeballCharacter`) 0.0 "VTBlend_Linear" 0.0 true))

(event `SetViewToEncounterCamera`
  (`self.SetViewTargetWithBlend` self (`self.EncounterCamera`) 0.2 "VTBlend_Linear" 0.0 true))

(event `self.ReceivePossess`
  (params (PossessedPawn :type "Pawn Object Reference"))
  (`KismetSystemLibrary.PrintString` (`KismetStringLibrary.Concat_StrStr` (`self.GetMyName`) (`KismetStringLibrary.Conv_ObjectToString` PossessedPawn))))

(event `Key|One`
  (params (Key :type "Key Structure"))
  (:`Released`
    (`self.SetViewToPawn` 0.0)))

(fn `UserConstructionScript`)